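; Bike Blueprint that links the vehicle's speed and steering values to its skeletal mesh animation.
; BeginPlay caches the bike's AnimBlueprint, and Tick copies CurrentSpeed and the MyFloatSteering result into it each frame.
; The look input events are empty, and the interpolated throttle, steering, lean and movement logic, along with camera rotation nodes, is left disconnected and never runs.
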(event EventBeginPlay
  (bind _asveh_bike_01_anim_blueprint (Utilities|Casting|CastToSKEL_Veh_Bike_01_AnimBlueprint (Components|SkeletalMesh|GetAnimInstance (Variables|Default|GetBikeMesh))))
  (Variables|Default|SetAs%20Veh%20Bike%2001%20Anim%20Blueprint _asveh_bike_01_anim_blueprint))

(event Collision|EventActorBeginOverlap
  (params (OtherActor :type Actor%20Object%20Reference)))

(event EventTick
  (params (DeltaSeconds :type Float%20%28single-precision%29))
  (bind _as_veh_bike_01_anim_blueprint (Variables|Default|GetAs%20Veh%20Bike%2001%20Anim%20Blueprint))
  (Variables|/Game/Polygon_BattleRoyale/Meshes/Vehicles/SKEL_Veh_Bike_01_AnimBlueprint.SKEL_Veh_Bike_01_AnimBlueprint_C|SetSpeed _as_veh_bike_01_anim_blueprint (Variables|Default|GetCurrentSpeed))
  (bind _returnvalue (Class|Bike|MyFloatSteering))
  (Variables|/Game/Polygon_BattleRoyale/Meshes/Vehicles/SKEL_Veh_Bike_01_AnimBlueprint.SKEL_Veh_Bike_01_AnimBlueprint_C|SetSteering _as_veh_bike_01_anim_blueprint _returnvalue))

(event Input|AxisEvents|InputAxisLookUp
  (params (AxisValue :type Float%20%28single-precision%29)))

(event Input|AxisEvents|InputAxisLookRight
  (params (AxisValue :type Float%20%28single-precision%29)))

(fn ConstructionScript)